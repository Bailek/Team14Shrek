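; Boss actor that cycles through colour materials and takes damage from Gift actors matching its current colour ID.
; Tick uses a Delay as a timer, then IndexOfMaterial finds the current material by display name and returns the next, wrapping around, with its index as Id.
; On Hit, a CheckID match calls DestroyActor immediately, then decrements Health, prints remaining life in French and destroys again at zero.
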(event `self.ReceiveBeginPlay`
  ;[1 1 1] Change RunTime Material
)

(event `self.ReceiveTick`
  (params (DeltaSeconds :type "Float (single-precision)"))
  ;[1 1 1] Change RunTime Material
  (`KismetSystemLibrary.Delay` (`self.colorDelay`))
  (bind (_newmaterial _newid) (`self.IndexOf Material`))
  (set `self.id` _newid)
  (`PrimitiveComponent.SetMaterial` (`self.StaticMesh`) 0 _newmaterial))

(event `self.ReceiveHit`
  (params (MyComp :type "PrimitiveComponent Object Reference") (Other :type "Actor Object Reference") (OtherComp :type "PrimitiveComponent Object Reference") (bSelfMoved :type Boolean) (HitLocation :type "Vector Structure") (HitNormal :type "Vector Structure") (NormalImpulse :type "Vector Structure") (Hit :type "HitResult Structure (by ref)"))
  ;[1 1 1] Boss Damage
  (bind _asgift (cast `/Game/AM/BP/Gift` Other))
  (bind _issame (`self.Check ID` (`self.id`) (`/Game/AM/BP/Gift.id` _asgift)))
  (if _issame
    (`self.K2_DestroyActor`)
    (bind _result (`/Engine/EditorBlueprintResources/StandardMacros.DecrementInt` (`self.health`))
      (:`  `
        (bind _output_get (set `self.health` _result))
        (`|ExecutionSequence`
          (:`then_0`
            (`KismetSystemLibrary.PrintString` (`KismetStringLibrary.Concat_StrStr` "Il reste " (`KismetStringLibrary.Conv_IntToString` _output_get) " points de vie ")))
          (:`then_1`
            (if (<= (`self.health`) 0)
              (`self.K2_DestroyActor`))))))))

(fn `IndexOf Material`
  (returns (newMaterial :type "Material Object Reference") (newId :type Integer))
  (locals (currentIndex :type Integer))
  (bind _currentindex (`local.currentIndex`))
  (for (_array_element _array_index) (`self.mat`)
    (set `local.currentIndex` _array_index)
    (if (`KismetStringLibrary.EqualEqual_StrStr` (`KismetSystemLibrary.GetDisplayName` _array_element) (`KismetSystemLibrary.GetDisplayName` (`|GetArrayItem` (`MeshComponent.GetMaterials` (`self.StaticMesh`)))))
      (bind _output_get (set `local.currentIndex` (+ (`local.currentIndex`) 1)))
      (if (< _output_get (`KismetArrayLibrary.Array_Length` (`self.mat`)))
        (return (`|GetArrayItem` (`self.mat`) _currentindex) _currentindex)
        (else
          (return (`|GetArrayItem` (`self.mat`)) 0))))))

(fn `UserConstructionScript`)